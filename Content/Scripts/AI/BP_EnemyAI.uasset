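; Enemy robot AI character for Ascend, with an EMP bar, a detection meter and a switch that lets the player disable it.
; BeginPlay saves the spawn transform, links both widgets to the robot, hides the EMP bar and sets walk speed by PC or PCVR platform.
; Switch overlaps set the disable flag and enemy reference on the matching player pawn.
; UpdateAIState only stores the state, with no behavior logic here.
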(event OnComponentBeginOverlap(Switch)
  (params (OverlappedComponent :type Primitive%20Component%20Object%20Reference) (OtherActor :type Actor%20Object%20Reference) (OtherComp :type Primitive%20Component%20Object%20Reference) (OtherBodyIndex :type Integer) (bFromSweep :type Boolean) (SweepResult :type Hit%20Result%20Structure%20%28by%20ref%29))
  (bind _vrpawn (Variables|Default|GetVRPawn))
  (bind _bpfirstpersoncharacter (Variables|Default|GetBPFirstPersonCharacter))
  ;[0.05127 0.05127 0.05127] Enemy Switch Trigger (On Component Begin Overlap) To Change CanDisableRobot = True, So That The Player Can Interact With The Switch Behind The Robot To Disable Them
  (switch Utilities|FlowControl|Switch|SwitchonTargetPlatform (Variables|/Game/Scripts/Common/GI_Ascend.GI_Ascend_C|GetTargetPlatform (Variables|Default|GetGIAscend))
    (:NewEnumerator1
      (if (== OtherActor _bpfirstpersoncharacter)
        (Variables|/Game/Scripts/FirstPerson/Blueprints/BP_FirstPersonCharacter.BP_FirstPersonCharacter_C|SetCanDisableRobot? _bpfirstpersoncharacter true)
        (Variables|/Game/Scripts/FirstPerson/Blueprints/BP_FirstPersonCharacter.BP_FirstPersonCharacter_C|SetEnemyActor _bpfirstpersoncharacter self)
        (Variables|/Game/Scripts/FirstPerson/Blueprints/BP_FirstPersonCharacter.BP_FirstPersonCharacter_C|SetInstructions_T _bpfirstpersoncharacter (Variables|Default|GetInstructions_T))))
    (:NewEnumerator2
      (if (== OtherActor _vrpawn)
        (Variables|/Game/Scripts/VRTemplate/Blueprints/VRPawn.VRPawn_C|SetCanDisableRobot? _vrpawn true)
        (Variables|/Game/Scripts/VRTemplate/Blueprints/VRPawn.VRPawn_C|SetEnemyActor _vrpawn self)))))

(event OnComponentEndOverlap(Switch)
  (params (OverlappedComponent :type Primitive%20Component%20Object%20Reference) (OtherActor :type Actor%20Object%20Reference) (OtherComp :type Primitive%20Component%20Object%20Reference) (OtherBodyIndex :type Integer))
  (bind _vrpawn (Variables|Default|GetVRPawn))
  (bind _bpfirstpersoncharacter (Variables|Default|GetBPFirstPersonCharacter))
  ;[0.05127 0.05127 0.05127] Enemy Switch Trigger (On Component Begin Overlap) To Change CanDisableRobot = True, So That The Player Can Interact With The Switch Behind The Robot To Disable Them
  (switch Utilities|FlowControl|Switch|SwitchonTargetPlatform (Variables|/Game/Scripts/Common/GI_Ascend.GI_Ascend_C|GetTargetPlatform (Variables|Default|GetGIAscend))
    (:NewEnumerator1
      (if (== OtherActor _bpfirstpersoncharacter)
        (Variables|/Game/Scripts/FirstPerson/Blueprints/BP_FirstPersonCharacter.BP_FirstPersonCharacter_C|SetCanDisableRobot? _bpfirstpersoncharacter false)
        (Variables|/Game/Scripts/FirstPerson/Blueprints/BP_FirstPersonCharacter.BP_FirstPersonCharacter_C|SetEnemyActor _bpfirstpersoncharacter 0)
        (Variables|/Game/Scripts/FirstPerson/Blueprints/BP_FirstPersonCharacter.BP_FirstPersonCharacter_C|SetInstructions_T _bpfirstpersoncharacter "")))
    (:NewEnumerator2
      (if (== OtherActor _vrpawn)
        (Variables|/Game/Scripts/VRTemplate/Blueprints/VRPawn.VRPawn_C|SetCanDisableRobot? _vrpawn false)
        (Variables|/Game/Scripts/VRTemplate/Blueprints/VRPawn.VRPawn_C|SetEnemyActor _vrpawn self)))))

(event EventBeginPlay
  (bind _returnvalue (Game|GetPlayerCharacter 0))
  (bind _self self)
  (bind _detectionmeter (Variables|Default|GetDetectionMeter))
  (bind _charactermovement (Variables|Character|GetCharacterMovement))
  (bind _emp (Variables|Default|GetEMP))
  ;[0.05127 0.05127 0.05127] BeginPlay - Initializing Game Instance, Saving AI's Initial Location, Setting Up Default Values Like EMP & Walk Speeds
  (Variables|Default|SetAIInitialLocation (Transformation|GetActorLocation))
  (Variables|Default|SetAIInitialRotation (Transformation|GetActorRotation))
  (bind _asgi_ascend (Utilities|Casting|CastToGI_Ascend (Game|GetGameInstance)))
  (Variables|Default|SetGIAscend _asgi_ascend)
  (Variables|Default|SetCurrentEMP 0.0)
  (Variables|Default|SetMaxEMP 1e+02)
  (bind _asui_ai_empbar (Utilities|Casting|CastToUI_AI_EMPBar (UserInterface|GetUserWidgetObject _emp)))
  (Variables|/Game/Scripts/AI/UI_AI_EMPBar.UI_AI_EMPBar_C|SetOwner _asui_ai_empbar _self)
  (bind _asui_detection_meter (Utilities|Casting|CastToUI_DetectionMeter (UserInterface|GetUserWidgetObject (Variables|Default|GetDetectionMeter))))
  (Variables|/Game/Scripts/AI/UI_DetectionMeter.UI_DetectionMeter_C|SetOwner _asui_detection_meter _self)
  (Rendering|SetVisibility _emp false false)
  (Variables|Default|SetDetectionBarValue 0.0)
  (switch Utilities|FlowControl|Switch|SwitchonTargetPlatform (Variables|/Game/Scripts/Common/GI_Ascend.GI_Ascend_C|GetTargetPlatform (Variables|Default|GetGIAscend))
    (:NewEnumerator1
      (bind _asbp_first_person_character (Utilities|Casting|CastToBP_FirstPersonCharacter _returnvalue))
      (Variables|Default|SetBPFirstPersonCharacter _asbp_first_person_character)
      (Class|WidgetComponent|SetWidgetSpace _detectionmeter "World")
      (Variables|/Script/Engine.CharacterMovementComponent|SetMaxWalkSpeed _charactermovement 3.5e+02))
    (:NewEnumerator2
      (bind _asvrpawn (Utilities|Casting|CastToVRPawn _returnvalue))
      (Variables|Default|SetVRPawn _asvrpawn)
      (Class|WidgetComponent|SetWidgetSpace _detectionmeter "World")
      (Variables|/Script/Engine.CharacterMovementComponent|SetMaxWalkSpeed _charactermovement 2e+02))))

(fn ConstructionScript)

(fn UpdateAIState
  (params (AIState :type AIState%20Enum :default "NewEnumerator0"))
  (bind _output_get (Variables|Default|SetAIState AIState))
  (return _output_get))